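; Actor Blueprint that runs a 15-minute game countdown and quits the game when time runs out.
; On BeginPlay it creates the HUB widget, adds it to the viewport and starts a looping one-second timer.
; TimerPlay decrements the count and writes it to the widget.
; Tick polls for zero, shows the "Perdu" (lost) end text and quits after a short delay.
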(event `self.ReceiveBeginPlay`
  (bind _returnvalue (`|GenericCreateObject` "/Game/Blueprints/HUB.HUB_C" (`self.GetOwner`)))
  (`UserWidget.AddToViewport` _returnvalue 0)
  (set `self.ViewPort` _returnvalue)
  (set `self.Timer` 900.0)
  (`KismetSystemLibrary.K2_SetTimer` null "TimerPlay" 1.0 true))

(event `self.ReceiveTick`
  (params (DeltaSeconds :type "Float (single-precision)"))
  (if (<= (`self.Timer`) 0.0)
    (`self.SetTextenf` "Perdu")
    (`KismetSystemLibrary.Delay` 1.0)
    (`KismetSystemLibrary.QuitGame` null "Quit")))

(fn `SetTextenf`
  (params (TextDeFin :type Text))
  (set `/Game/Blueprints/HUB.TextEnd` TextDeFin (`self.ViewPort`)))

(fn `TimerPlay`
  (bind _output_get (set `self.Timer` (- (`self.Timer`) 1.0)))
  (set `/Game/Blueprints/HUB.Timer` (`KismetTextLibrary.Conv_StringToText` (`KismetStringLibrary.Conv_DoubleToString` _output_get)) (`self.ViewPort`)))

(fn `UserConstructionScript`)