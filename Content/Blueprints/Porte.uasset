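; Weight-activated door that moves vertically when a heavy enough component overlaps its Collison trigger.
; On begin overlap, a mass check either plays the DoorAnimation timeline or prints a "not enough weight" message in French.
; End overlap plays a second timeline, Timeline_0, without any mass check.
; Both timelines feed their DoorOpen track into the world Z location of ImagePorte.
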(event `self.Collison.OnComponentBeginOverlap`
  (params (OverlappedComponent :type "PrimitiveComponent Object Reference") (OtherActor :type "Actor Object Reference") (OtherComp :type "PrimitiveComponent Object Reference") (OtherBodyIndex :type Integer) (bFromSweep :type Boolean) (SweepResult :type "HitResult Structure (by ref)"))
  (if (>= (`PrimitiveComponent.GetMass` OtherComp) 655.0)
    (bind (_direction _dooropen) (`Timeline|DoorAnimation`)
      (:`Update`
        (`SceneComponent.K2_SetWorldLocation` (`self.ImagePorte`) (`KismetMathLibrary.MakeVector` 0.0 0.0 _dooropen) false false)))
    (else
      (`KismetSystemLibrary.PrintString` "Pas Assez de poiids"))))

(event `self.Collison.OnComponentEndOverlap`
  (params (OverlappedComponent :type "PrimitiveComponent Object Reference") (OtherActor :type "Actor Object Reference") (OtherComp :type "PrimitiveComponent Object Reference") (OtherBodyIndex :type Integer))
  (bind (_direction _dooropen) (`Timeline|Timeline_0`)
    (:`Update`
      (`SceneComponent.K2_SetWorldLocation` (`self.ImagePorte`) (`KismetMathLibrary.MakeVector` 0.0 0.0 _dooropen) false false))))

(fn `UserConstructionScript`)