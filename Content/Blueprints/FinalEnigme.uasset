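; FinalEnigme is the final puzzle actor: a two-pan balance scale, plus a trigger that ends the game.
; Left and right overlap volumes keep mass totals, adding only components up to a mass limit but subtracting any that leave.
; Tick sets each pan's height from the mass difference, lowering the heavier side.
; When an actor with a PhysicsHandle enters Box, the HUD shows "Victoire" and the game quits after a short delay.
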(event `self.ReceiveBeginPlay`)

(event `self.ReceiveTick`
  (params (DeltaSeconds :type "Float (single-precision)"))
  (bind _balancegauche (`self.BalanceGauche`))
  (bind _balancedroite (`self.BalanceDroite`))
  (bind _totalmassgauche (`self.TotalMassGauche`))
  (bind _totalmassdroite (`self.TotalMassDroite`))
  (bind (_returnvalue_x _returnvalue_y) (`KismetMathLibrary.BreakVector` (`SceneComponent.K2_GetComponentLocation` _balancegauche)))
  (bind (_returnvalue_x_2 _returnvalue_y_2) (`KismetMathLibrary.BreakVector` (`SceneComponent.K2_GetComponentLocation` _balancedroite)))
  ;[1 1 1] Debug Total mass
  ;[1 1 1] Balancier
  (`SceneComponent.K2_SetWorldLocation` _balancedroite (`KismetMathLibrary.MakeVector` _returnvalue_x_2 _returnvalue_y_2 (+ -480.0 (/ (- _totalmassdroite _totalmassgauche) -26.0))) false false)
  (`SceneComponent.K2_SetWorldLocation` _balancegauche (`KismetMathLibrary.MakeVector` _returnvalue_x _returnvalue_y (+ -480.0 (/ (- _totalmassgauche _totalmassdroite) -26.0))) false false))

(event `self.Droite.OnComponentBeginOverlap`
  (params (OverlappedComponent :type "PrimitiveComponent Object Reference") (OtherActor :type "Actor Object Reference") (OtherComp :type "PrimitiveComponent Object Reference") (OtherBodyIndex :type Integer) (bFromSweep :type Boolean) (SweepResult :type "HitResult Structure (by ref)"))
  (bind _returnvalue (`PrimitiveComponent.GetMass` OtherComp))
  ;[1 1 1] Gestion Poids
  (if (<= _returnvalue 1000.0)
    (set `self.TotalMassDroite` (+ (`self.TotalMassDroite`) _returnvalue))))

(event `self.Gauche.OnComponentBeginOverlap`
  (params (OverlappedComponent :type "PrimitiveComponent Object Reference") (OtherActor :type "Actor Object Reference") (OtherComp :type "PrimitiveComponent Object Reference") (OtherBodyIndex :type Integer) (bFromSweep :type Boolean) (SweepResult :type "HitResult Structure (by ref)"))
  (bind _returnvalue (`PrimitiveComponent.GetMass` OtherComp))
  ;[1 1 1] Gestion Poids
  (if (<= _returnvalue 1000.0)
    (set `self.TotalMassGauche` (+ (`self.TotalMassGauche`) _returnvalue))))

(event `self.Gauche.OnComponentEndOverlap`
  (params (OverlappedComponent :type "PrimitiveComponent Object Reference") (OtherActor :type "Actor Object Reference") (OtherComp :type "PrimitiveComponent Object Reference") (OtherBodyIndex :type Integer))
  ;[1 1 1] Gestion Poids
  (set `self.TotalMassGauche` (- (`self.TotalMassGauche`) (`PrimitiveComponent.GetMass` OtherComp))))

(event `self.Droite.OnComponentEndOverlap`
  (params (OverlappedComponent :type "PrimitiveComponent Object Reference") (OtherActor :type "Actor Object Reference") (OtherComp :type "PrimitiveComponent Object Reference") (OtherBodyIndex :type Integer))
  ;[1 1 1] Gestion Poids
  (set `self.TotalMassDroite` (- (`self.TotalMassDroite`) (`PrimitiveComponent.GetMass` OtherComp))))

(event `self.Box.OnComponentBeginOverlap`
  (params (OverlappedComponent :type "PrimitiveComponent Object Reference") (OtherActor :type "Actor Object Reference") (OtherComp :type "PrimitiveComponent Object Reference") (OtherBodyIndex :type Integer) (bFromSweep :type Boolean) (SweepResult :type "HitResult Structure (by ref)"))
  ;[1 1 1] Quit Game
  (if (`KismetSystemLibrary.IsValid` (`self.GetComponentByClass` OtherActor "/Script/Engine.PhysicsHandleComponent"))
    (bind _ashub_blue_print (cast `/Game/Blueprints/Hub_BluePrint` (`PlayerController.GetHUD` (`GameplayStatics.GetPlayerController` 0)))
      (:`then`
        (`/Game/Blueprints/Hub_BluePrint.SetTextenf` _ashub_blue_print "Victoire")
        (`KismetSystemLibrary.Delay` 1.0)
        (`KismetSystemLibrary.QuitGame` null "Quit"))
      (:`CastFailed`
        (`KismetSystemLibrary.QuitGame` null "Quit")))))

(fn `UserConstructionScript`)