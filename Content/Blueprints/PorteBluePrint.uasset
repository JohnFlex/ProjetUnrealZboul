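; Puzzle door Blueprint that opens when six trigger boxes are all in their correct weight states.
; Boxes 1, 3, 4 and 6 check the overlapping component's mass against a range or minimum, while 2 and 5 must stay empty.
; Tick checks the resulting flags and plays timelines that move ImagePorte's world Z.
; The close timeline plays only when Box6 fails with the other five satisfied.
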(event `self.ReceiveTick`
  (params (DeltaSeconds :type "Float (single-precision)"))
  ;[1 1 1] Can Open the door ?
  (if (`self.Box4OK`)
    (if (`self.Box5OK`)
      (if (`self.Box1OK`)
        (if (`self.Box2OK`)
          (if (`self.Box3OK`)
            (if (`self.Box6OK`)
              (bind (_direction _opendoor) (`Timeline|DoorOpen`)
                (:`Update`
                  (`SceneComponent.K2_SetWorldLocation` (`self.ImagePorte`) (`KismetMathLibrary.MakeVector` 0.0 0.0 _opendoor) false false)))
              (else
                (bind (_direction_2 _newtrack_0) (`Timeline|CloseDoor`)
                  (:`Update`
                    (`SceneComponent.K2_SetWorldLocation` (`self.ImagePorte`) (`KismetMathLibrary.MakeVector` 0.0 0.0 _newtrack_0) false false)))))))))))

(event `self.1.OnComponentBeginOverlap`
  (params (OverlappedComponent :type "PrimitiveComponent Object Reference") (OtherActor :type "Actor Object Reference") (OtherComp :type "PrimitiveComponent Object Reference") (OtherBodyIndex :type Integer) (bFromSweep :type Boolean) (SweepResult :type "HitResult Structure (by ref)"))
  (bind _returnvalue (`PrimitiveComponent.GetMass` OtherComp))
  ;[1 1 1] Overlap One Block
  (if (>= _returnvalue 25.0)
    (if (<= _returnvalue 30.0)
      (set `self.Box1OK` true))))

(event `self.1.OnComponentEndOverlap`
  (params (OverlappedComponent :type "PrimitiveComponent Object Reference") (OtherActor :type "Actor Object Reference") (OtherComp :type "PrimitiveComponent Object Reference") (OtherBodyIndex :type Integer))
  ;[1 1 1] Set END overlap block
  (set `self.Box1OK` false))

(event `self.2.OnComponentBeginOverlap`
  (params (OverlappedComponent :type "PrimitiveComponent Object Reference") (OtherActor :type "Actor Object Reference") (OtherComp :type "PrimitiveComponent Object Reference") (OtherBodyIndex :type Integer) (bFromSweep :type Boolean) (SweepResult :type "HitResult Structure (by ref)"))
  ;[1 1 1] Overlap One Block
  (if (>= (`PrimitiveComponent.GetMass` OtherComp) 0.0)
    (set `self.Box2OK` false)))

(event `self.2.OnComponentEndOverlap`
  (params (OverlappedComponent :type "PrimitiveComponent Object Reference") (OtherActor :type "Actor Object Reference") (OtherComp :type "PrimitiveComponent Object Reference") (OtherBodyIndex :type Integer))
  ;[1 1 1] Set END overlap block
  (set `self.Box2OK` true))

(event `self.3.OnComponentBeginOverlap`
  (params (OverlappedComponent :type "PrimitiveComponent Object Reference") (OtherActor :type "Actor Object Reference") (OtherComp :type "PrimitiveComponent Object Reference") (OtherBodyIndex :type Integer) (bFromSweep :type Boolean) (SweepResult :type "HitResult Structure (by ref)"))
  (bind _returnvalue (`PrimitiveComponent.GetMass` OtherComp))
  ;[1 1 1] Overlap One Block
  (if (>= _returnvalue 75.0)
    (if (<= _returnvalue 80.0)
      (set `self.Box3OK` true))))

(event `self.3.OnComponentEndOverlap`
  (params (OverlappedComponent :type "PrimitiveComponent Object Reference") (OtherActor :type "Actor Object Reference") (OtherComp :type "PrimitiveComponent Object Reference") (OtherBodyIndex :type Integer))
  ;[1 1 1] Set END overlap block
  (set `self.Box3OK` false))

(event `self.4.OnComponentBeginOverlap`
  (params (OverlappedComponent :type "PrimitiveComponent Object Reference") (OtherActor :type "Actor Object Reference") (OtherComp :type "PrimitiveComponent Object Reference") (OtherBodyIndex :type Integer) (bFromSweep :type Boolean) (SweepResult :type "HitResult Structure (by ref)"))
  (bind _returnvalue (`PrimitiveComponent.GetMass` OtherComp))
  ;[1 1 1] Overlap One Block
  (if (>= _returnvalue 30.0)
    (if (<= _returnvalue 35.0)
      (set `self.Box4OK` true))))

(event `self.4.OnComponentEndOverlap`
  (params (OverlappedComponent :type "PrimitiveComponent Object Reference") (OtherActor :type "Actor Object Reference") (OtherComp :type "PrimitiveComponent Object Reference") (OtherBodyIndex :type Integer))
  ;[1 1 1] Set END overlap block
  (set `self.Box4OK` false))

(event `self.5.OnComponentBeginOverlap`
  (params (OverlappedComponent :type "PrimitiveComponent Object Reference") (OtherActor :type "Actor Object Reference") (OtherComp :type "PrimitiveComponent Object Reference") (OtherBodyIndex :type Integer) (bFromSweep :type Boolean) (SweepResult :type "HitResult Structure (by ref)"))
  ;[1 1 1] Overlap One Block
  (if (>= (`PrimitiveComponent.GetMass` OtherComp) 0.0)
    (set `self.Box5OK` false)))

(event `self.5.OnComponentEndOverlap`
  (params (OverlappedComponent :type "PrimitiveComponent Object Reference") (OtherActor :type "Actor Object Reference") (OtherComp :type "PrimitiveComponent Object Reference") (OtherBodyIndex :type Integer))
  ;[1 1 1] Set END overlap block
  (set `self.Box5OK` true))

(event `self.6.OnComponentBeginOverlap`
  (params (OverlappedComponent :type "PrimitiveComponent Object Reference") (OtherActor :type "Actor Object Reference") (OtherComp :type "PrimitiveComponent Object Reference") (OtherBodyIndex :type Integer) (bFromSweep :type Boolean) (SweepResult :type "HitResult Structure (by ref)"))
  (bind _returnvalue (`PrimitiveComponent.GetMass` OtherComp))
  ;[1 1 1] Overlap One Block
  (if (>= _returnvalue 120.0)
    (if (<= 0.0 _returnvalue)
      (set `self.Box6OK` true))))

(event `self.6.OnComponentEndOverlap`
  (params (OverlappedComponent :type "PrimitiveComponent Object Reference") (OtherActor :type "Actor Object Reference") (OtherComp :type "PrimitiveComponent Object Reference") (OtherBodyIndex :type Integer))
  ;[1 1 1] Set END overlap block
  (set `self.Box6OK` false))

(fn `UserConstructionScript`)