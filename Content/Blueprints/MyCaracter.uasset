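; First-person style player character Blueprint with axis-driven movement and look, jumping, and physics object grabbing.
; SuperJump temporarily raises the max jump count and calls Jump twice, restoring the count on release.
; Grab line-traces from the camera for physics bodies, with persistent debug drawing, and attaches hits to a PhysicsHandle.
; Tick holds the target ahead of the camera; releasing Grab only clears the flag, without releasing the component.
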(event `InputAxis|MouseUp`
  (params (AxisValue :type "Float (single-precision)"))
  ;[1 1 1] Cam Move
  (`self.AddControllerPitchInput` AxisValue))

(event `self.ReceiveTick`
  (params (DeltaSeconds :type "Float (single-precision)"))
  (bind _mycam (`self.MyCam`))
  (if (`self.Grab`)
    (`PhysicsHandleComponent.SetTargetLocation` (`self.PhysicsHandle`) (+ (`SceneComponent.K2_GetComponentLocation` _mycam) (* (`KismetMathLibrary.GetForwardVector` (`SceneComponent.K2_GetComponentRotation` _mycam)) 150.0)))))

(event `InputAxis|MouseRight`
  (params (AxisValue :type "Float (single-precision)"))
  ;[1 1 1] Cam Move
  (`self.AddControllerYawInput` AxisValue))

(event `InputAction|Jump`
  (params (Key :type "Key Structure"))
  (:`Pressed`
    (`self.Jump`)))

(event `InputAxis|Profondeur`
  (params (AxisValue :type "Float (single-precision)"))
  ;[1 1 1] PlayerMove
  (`self.AddMovementInput` (`self.GetActorForwardVector`) AxisValue))

(event `InputAction|SuperJump`
  (params (Key :type "Key Structure"))
  (:`Pressed`
    (set `self.JumpMaxCount` 2)
    (`self.Jump`)
    (`self.Jump`))
  (:`Released`
    (set `self.JumpMaxCount` 1)))

(event `InputAxis|Largeur`
  (params (AxisValue :type "Float (single-precision)"))
  ;[1 1 1] PlayerMove
  (`self.AddMovementInput` (`self.GetActorRightVector`) AxisValue))

(event `InputAction|Grab`
  (params (Key :type "Key Structure"))
  (bind _mycam (`self.MyCam`))
  (bind _returnvalue (`SceneComponent.K2_GetComponentLocation` _mycam))
  (:`Pressed`
    (bind (_outhit _returnvalue_2) (`KismetSystemLibrary.LineTraceSingleForObjects` :`Start` _returnvalue :`End` (+ _returnvalue (* (`KismetMathLibrary.GetForwardVector` (`SceneComponent.K2_GetComponentRotation` _mycam)) 500.0)) :`ObjectTypes` (`|MakeArray` "ObjectTypeQuery4" :!type "EObjectTypeQuery Enum") :`DrawDebugType` "Persistent" :`DrawTime` 10.0))
    (if _returnvalue_2
      (bind (_bblockinghit _binitialoverlap _time _distance _location _impactpoint _normal _impactnormal _physmat _hitactor _hitcomponent) (`GameplayStatics.BreakHitResult` _outhit))
      (`PhysicsHandleComponent.GrabComponentAtLocation` (`self.PhysicsHandle`) _hitcomponent "None" _location)
      (set `self.Grab` true)))
  (:`Released`
    (set `self.Grab` false)))

(fn `UserConstructionScript`)